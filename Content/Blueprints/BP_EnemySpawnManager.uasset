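; BP_EnemySpawnManager populates the level at BeginPlay with randomized BP_AiMoveTo AI characters.
; It finds every BP_EnemySpawnPoint, prints the count, and spawns an AI at each with a random coin flip, owned by that point.
; Each spawn gets its name text, two materials and skeletal mesh by shuffling the Names, Materials and SkeletalMeshes arrays and taking the first entries.
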(event EventBeginPlay
  (bind _names (Variables|Default|GetNames))
  (bind _skeletalmeshes (Variables|Default|GetSkeletalMeshes))
  (bind _materials (Variables|Default|GetMaterials))
  (bind _outactors (Actor|GetAllActorsOfClass "/Game/Blueprints/BP_EnemySpawnPoint.BP_EnemySpawnPoint_C"))
  (Development|PrintText (Utilities|Text|FormatText "{count} spawn points initialized." (Utilities|Array|Length _outactors)) true true "(R=1.000000,G=0.102098,B=0.895091,A=1.000000)" 5.0)
  (for _array_element _outactors
    (if (Math|Random|RandomBool)
      (bind _returnvalue (Game|SpawnActorfromClass "/Game/AI_Blueprints/BP_AiMoveTo.BP_AiMoveTo_C" (Transformation|GetActorTransform _array_element) "Undefined" "MultiplyWithRoot" _array_element 0))
      ;[0.15 0.15 0.15 0.5] Shuffle name array then select the first index.
      (Utilities|Array|Shuffle _names)
      (Rendering|Components|TextRender|SetText (Variables|/Game/AI_Blueprints/BP_AiMoveTo.BP_AiMoveTo_C|GetAI%20Name%20Text _returnvalue) (Utilities|Array|Get(acopy) _names))
      ;[0.15 0.15 0.15 0.5] Shuffle Material array and set the AI materials to the first and second index.
      (Utilities|Array|Shuffle _materials)
      (Rendering|Material|SetMaterial (Variables|/Script/Engine.Character|GetMesh _returnvalue) 0 (Utilities|Array|Get(acopy) _materials))
      (Rendering|Material|SetMaterial (Variables|/Script/Engine.Character|GetMesh _returnvalue) 1 (Utilities|Array|Get(acopy) _materials 1))
      ;[0.15 0.15 0.15 0.5] Shuffle an array of Skeletal Meshes and set the AI SM to the first index.
      (Utilities|Array|Shuffle _skeletalmeshes)
      (Components|SkeletalMesh|SetSkeletalMeshAsset (Variables|/Script/Engine.Character|GetMesh _returnvalue) (Utilities|Array|Get(acopy) _skeletalmeshes)))))

(fn ConstructionScript)