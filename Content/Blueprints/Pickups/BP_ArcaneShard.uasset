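; BP_ArcaneShard is a collectible shard pickup that records its collection in the level's save state.
; When BP_ThirdPersonCharacter overlaps its mesh, it adds itself to GM_SaveLoad's SGLevelState AlteredActors list, plays a crystal collect sound and destroys itself.
; Its LoadState event calls AlreadyCollected, which swaps the mesh to a Glass material rather than removing the actor.
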(event OnComponentBeginOverlap(Mesh)
  (params (OverlappedComponent :type Primitive%20Component%20Object%20Reference) (OtherActor :type Actor%20Object%20Reference) (OtherComp :type Primitive%20Component%20Object%20Reference) (OtherBodyIndex :type Integer) (bFromSweep :type Boolean) (SweepResult :type Hit%20Result%20Structure%20%28by%20ref%29))
  (Utilities|Casting|CastToBP_ThirdPersonCharacter OtherActor)
  (bind _asgm_save_load (Utilities|Casting|CastToGM_SaveLoad (Game|GetGameMode)))
  (Utilities|Array|AddUnique (Variables|/Game/Blueprints/Saving/SG_LevelState.SG_LevelState_C|GetAlteredActors (Variables|/Game/Blueprints/Saving/GM_SaveLoad.GM_SaveLoad_C|GetSG_LevelState _asgm_save_load)) self)
  (Audio|PlaySoundatLocation "/Game/Audio/Item/crystalCollect_Cue.crystalCollect_Cue" (Transformation|GetActorLocation) "0, 0, 0" 1.0 1.0 0.0 0 0 0 0)
  (Actor|DestroyActor))

(event Custom|AlreadyCollected
  (Rendering|Material|SetMaterial (Variables|Default|GetMesh) 0 "/DatasmithContent/Materials/FBXImporter/VRED/Glass.Glass"))

(event EventLoadState
  (CallFunction|AlreadyCollected))

(fn ConstructionScript)