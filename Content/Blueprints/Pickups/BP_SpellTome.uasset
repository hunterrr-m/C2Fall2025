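; BP_SpellTome is a pickup spell book that attaches to a skeletal mesh socket when held and drops back into physics.
; Primary and secondary use spend mana and fire the player character's normal or advanced projectile, the latter costing more.
; Each spell has its own Delay-based cooldown and HUD timer, which start even if mana is insufficient.
; The player is cached at BeginPlay from player index 0.
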(event Custom|StartSpellCooldown
  (Variables|Default|SetOnCooldown? true)
  (Default|StartTimer (Variables|/Game/ThirdPerson/Blueprints/BP_ThirdPersonCharacter.BP_ThirdPersonCharacter_C|GetSpellSlots (Variables|Default|GetPlayer)))
  (Utilities|FlowControl|Delay 3.0)
  (Variables|Default|SetOnCooldown? false))

(event Custom|StartAdvSpellCooldown
  (Variables|Default|SetAdvOnCooldown? true)
  (Default|StartAdvTimer (Variables|/Game/ThirdPerson/Blueprints/BP_ThirdPersonCharacter.BP_ThirdPersonCharacter_C|GetSpellSlots (Variables|Default|GetPlayer)))
  (Utilities|FlowControl|Delay 6.0)
  (Variables|Default|SetAdvOnCooldown? false))

(event EventBeginPlay
  (bind _asbp_third_person_character (Utilities|Casting|CastToBP_ThirdPersonCharacter (Game|GetPlayerCharacter 0)))
  (Variables|Default|SetPlayer _asbp_third_person_character))

(event EventUseSecondary
  (bind _player (Variables|Default|GetPlayer))
  (if (not (Variables|Default|GetAdvOnCooldown?))
    (CallFunction|StartAdvSpellCooldown)
    (if (>= (Variables|/Game/ThirdPerson/Blueprints/BP_ThirdPersonCharacter.BP_ThirdPersonCharacter_C|GetMana (Variables|Default|GetPlayer)) 2e+01)
      (Variables|/Game/ThirdPerson/Blueprints/BP_ThirdPersonCharacter.BP_ThirdPersonCharacter_C|SetMana _player (- (Variables|/Game/ThirdPerson/Blueprints/BP_ThirdPersonCharacter.BP_ThirdPersonCharacter_C|GetMana (Variables|Default|GetPlayer)) 2e+01))
      (Default|UpdateMana (Variables|/Game/ThirdPerson/Blueprints/BP_ThirdPersonCharacter.BP_ThirdPersonCharacter_C|GetW_BarStats _player))
      (Default|ShootProjectile _player true))))

(event EventPickup
  (params (SKMesh :type Skeletal%20Mesh%20Component%20Object%20Reference) (Parent :type BP%20Third%20Person%20Character%20Object%20Reference))
  (Transformation|AttachComponentToComponent SKMesh "BPI_item_socket" "SnapToTarget" "SnapToTarget" "SnapToTarget" true)
  (Physics|SetSimulatePhysics (Variables|Default|GetMesh) false)
  (Collision|SetCollisionEnabled (Variables|Default|GetMesh) "NoCollision")
  (Collision|SetCollisionEnabled (Variables|Default|GetCollision) "NoCollision"))

(event EventUsePrimary
  (bind _player (Variables|Default|GetPlayer))
  (if (not (Variables|Default|GetOnCooldown?))
    (CallFunction|StartSpellCooldown)
    (if (>= (Variables|/Game/ThirdPerson/Blueprints/BP_ThirdPersonCharacter.BP_ThirdPersonCharacter_C|GetMana (Variables|Default|GetPlayer)) 1e+01)
      (Variables|/Game/ThirdPerson/Blueprints/BP_ThirdPersonCharacter.BP_ThirdPersonCharacter_C|SetMana _player (- (Variables|/Game/ThirdPerson/Blueprints/BP_ThirdPersonCharacter.BP_ThirdPersonCharacter_C|GetMana (Variables|Default|GetPlayer)) 1e+01))
      (Default|UpdateMana (Variables|/Game/ThirdPerson/Blueprints/BP_ThirdPersonCharacter.BP_ThirdPersonCharacter_C|GetW_BarStats _player))
      (Default|ShootProjectile _player false))))

(event EventDrop
  (params (PlayerRef :type BP%20Third%20Person%20Character%20Object%20Reference))
  (Transformation|DetachFromComponent (Variables|Default|GetDefaultSceneRoot) "KeepWorld" "KeepWorld" "KeepWorld" true)
  (Physics|SetSimulatePhysics (Variables|Default|GetMesh) true)
  (Collision|SetCollisionEnabled (Variables|Default|GetMesh) "QueryAndPhysics")
  (Collision|SetCollisionEnabled (Variables|Default|GetCollision) "QueryOnly"))

(fn ConstructionScript)