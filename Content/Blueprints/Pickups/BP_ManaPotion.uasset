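; BP_ManaPotion is a held pickup item that restores the player's mana when used.
; It caches the third-person character on BeginPlay, and Pickup and Drop toggle physics and collision while attaching it to or detaching it from a hand-held item socket.
; Primary use destroys it, clears the held item, adds clamped mana and refreshes the stats widget.
; Secondary use does nothing, and being stolen simply destroys it.
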(event EventBeginPlay
  (bind _asbp_third_person_character (Utilities|Casting|CastToBP_ThirdPersonCharacter (Game|GetPlayerCharacter 0)))
  (Variables|Default|SetPlayer _asbp_third_person_character))

(event EventStolen
  (Actor|DestroyActor))

(event EventUseSecondary)

(event EventPickup
  (params (SKMesh :type Skeletal%20Mesh%20Component%20Object%20Reference) (Parent :type BP%20Third%20Person%20Character%20Object%20Reference))
  (Transformation|AttachComponentToComponent SKMesh "BPI_item_socket" "SnapToTarget" "SnapToTarget" "SnapToTarget" true)
  (Physics|SetSimulatePhysics (Variables|Default|GetMesh) false)
  (Collision|SetCollisionEnabled (Variables|Default|GetMesh) "NoCollision")
  (Collision|SetCollisionEnabled (Variables|Default|GetCollision) "NoCollision"))

(event EventUsePrimary
  (bind _player (Variables|Default|GetPlayer))
  (Actor|DestroyActor)
  (Variables|/Game/ThirdPerson/Blueprints/BP_ThirdPersonCharacter.BP_ThirdPersonCharacter_C|SetHeldItem _player 0)
  (Variables|/Game/ThirdPerson/Blueprints/BP_ThirdPersonCharacter.BP_ThirdPersonCharacter_C|SetMana _player (Math|Float|Clamp(Float) (+ (Variables|/Game/ThirdPerson/Blueprints/BP_ThirdPersonCharacter.BP_ThirdPersonCharacter_C|GetMana _player) 3e+01) 0.0 5e+01))
  (Default|UpdateMana (Variables|/Game/ThirdPerson/Blueprints/BP_ThirdPersonCharacter.BP_ThirdPersonCharacter_C|GetW_BarStats _player)))

(event EventDrop
  (params (PlayerRef :type BP%20Third%20Person%20Character%20Object%20Reference))
  (Transformation|DetachFromComponent (Variables|Default|GetDefaultSceneRoot) "KeepWorld" "KeepWorld" "KeepWorld" true)
  (Physics|SetSimulatePhysics (Variables|Default|GetMesh) true)
  (Collision|SetCollisionEnabled (Variables|Default|GetMesh) "QueryAndPhysics")
  (Collision|SetCollisionEnabled (Variables|Default|GetCollision) "QueryOnly"))

(fn ConstructionScript)