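; BP_SpeedMachine is a pickup item that lets the character holding it toggle speeding up or slowing down.
; Pickup stores the parent as CharacterRef, snaps the item to the mesh's BPI_item_socket and disables collision.
; Drop detaches it in world space and restores mesh and trigger collision.
; Primary and secondary use call SpeedUp and SlowDown on the character, which owns the speed logic; every event prints debug text.
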(event EventPickup
  (params (SKMesh :type Skeletal%20Mesh%20Component%20Object%20Reference) (Parent :type BP%20Third%20Person%20Character%20Object%20Reference))
  ;[0.15 0.15 0.15 0.5] Event Pickup
  (Development|PrintText "Pickup called on speed machine" true true "(R=1.000000,G=0.825543,B=0.000000,A=1.000000)")
  (Variables|Default|SetCharacter%20Ref Parent)
  (Transformation|AttachComponentToComponent SKMesh "BPI_item_socket" "SnapToTarget" "SnapToTarget" "KeepRelative" true)
  (Collision|SetCollisionEnabled (Variables|Default|GetMesh) "NoCollision")
  (Collision|SetCollisionEnabled (Variables|Default|GetCollision) "NoCollision"))

(event EventUsePrimary
  ;[0.15 0.15 0.15 0.5] Primary + Secondary Events
  (Development|PrintText "Toggle speed up")
  (Default|SpeedUp (Variables|Default|GetCharacter%20Ref)))

(event EventDrop
  ;[0.15 0.15 0.15 0.5] Event Drop
  (Development|PrintText "Drop called on speed machine." true true "(R=1.000000,G=0.856370,B=0.000000,A=1.000000)")
  (Transformation|DetachFromComponent (Variables|Default|GetDefaultSceneRoot) "KeepWorld" "KeepRelative" "KeepRelative" true)
  (Collision|SetCollisionEnabled (Variables|Default|GetMesh) "QueryAndPhysics")
  (Collision|SetCollisionEnabled (Variables|Default|GetCollision) "QueryOnly"))

(event EventUseSecondary
  ;[0.15 0.15 0.15 0.5] Primary + Secondary Events
  (Development|PrintText "Toggle slow down")
  (Default|SlowDown (Variables|Default|GetCharacter%20Ref)))

(fn ConstructionScript)