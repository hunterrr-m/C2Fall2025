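; BP_ElementalBarrier is a barrier that only lets the player pass when their elemental type matches the barrier's own.
; On BeginPlay its TextRender displays a label chosen from its ElementalType, one of eight elements.
; When a BP_ThirdPersonCharacter of the same type overlaps the Trigger, the Barrier component's collision is switched off.
; Nothing in the graph turns the collision back on, so the barrier stays passable afterwards.
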(event OnComponentBeginOverlap(Trigger)
  (params (OverlappedComponent :type Primitive%20Component%20Object%20Reference) (OtherActor :type Actor%20Object%20Reference) (OtherComp :type Primitive%20Component%20Object%20Reference) (OtherBodyIndex :type Integer) (bFromSweep :type Boolean) (SweepResult :type Hit%20Result%20Structure%20%28by%20ref%29))
  (bind _asbp_third_person_character (Utilities|Casting|CastToBP_ThirdPersonCharacter OtherActor))
  (if (Utilities|Enum|Equal(Enum) (Variables|/Game/ThirdPerson/Blueprints/BP_ThirdPersonCharacter.BP_ThirdPersonCharacter_C|GetelementalType _asbp_third_person_character) (Variables|Default|GetelementalType)) ; Does player type match barrier type?
    (Collision|SetCollisionEnabled (Variables|Default|GetBarrier) "NoCollision")))

(event EventBeginPlay
  (Rendering|Components|TextRender|SetText (Variables|Default|GetTextRender) (Utilities|Select :Index (Variables|Default|GetelementalType) :NewEnumerator0 "Basic Barrier" :NewEnumerator1 "Plasma Barrier" :NewEnumerator2 "Void Barrier" :NewEnumerator3 "Mirror Barrier" :NewEnumerator4 "Regolith Barrier" :NewEnumerator5 "Noise Barrier" :NewEnumerator6 "Mercury Barrier" :NewEnumerator7 "Gravity Barrier")))

(fn ConstructionScript)