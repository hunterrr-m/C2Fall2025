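; BP_KeyDoor is a locked door that opens when the third person character enters its trigger carrying a key.
; On overlap it checks the character's KeyCount, spends one key, and plays the Open timeline to swing the Door's yaw through up to 90 degrees.
; IsOpen is set during the timeline update to block further triggers, and a keyless player gets an on-screen debug message.
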(event OnComponentBeginOverlap(Trigger)
  (params (OverlappedComponent :type Primitive%20Component%20Object%20Reference) (OtherActor :type Actor%20Object%20Reference) (OtherComp :type Primitive%20Component%20Object%20Reference) (OtherBodyIndex :type Integer) (bFromSweep :type Boolean) (SweepResult :type Hit%20Result%20Structure%20%28by%20ref%29))
  (if (not (Variables|Default|GetisOpen?))
    (bind _asbp_third_person_character (Utilities|Casting|CastToBP_ThirdPersonCharacter OtherActor))
    (if (> (Variables|/Game/ThirdPerson/Blueprints/BP_ThirdPersonCharacter.BP_ThirdPersonCharacter_C|GetkeyCount _asbp_third_person_character) 0)
      (Math|Integer|DecrementInt (Variables|/Game/ThirdPerson/Blueprints/BP_ThirdPersonCharacter.BP_ThirdPersonCharacter_C|GetkeyCount _asbp_third_person_character)
        (:%20%20
          (bind _newtrack_0 (Timeline|Open Play)
            (:Update
              (Transformation|SetRelativeRotation (Variables|Default|GetDoor) (Math|Rotator|MakeRotator 0.0 0.0 (* _newtrack_0 9e+01)) false false)
              (Variables|Default|SetisOpen? true)))))
      (else
        (Development|PrintString "Player needs a key!" true true "(R=0.644792,G=0.000000,B=0.031956,A=1.000000)" 3.0)))))

(event EventBeginPlay)

(event Collision|EventActorBeginOverlap
  (params (OtherActor :type Actor%20Object%20Reference)))

(event EventTick
  (params (DeltaSeconds :type Float%20%28single-precision%29)))

(fn ConstructionScript)