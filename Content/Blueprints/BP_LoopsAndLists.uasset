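; BP_LoopsAndLists is a demo Blueprint of loop types and array access that prints its results as text.
; BeginPlay starts DelayLoop, a self-calling event throttled by Delay and capped by DoN, which fires the For loop on each pass.
; The For loop indexes into a list of green shades to color its text.
; While countdown and ForEach color events are also defined but not called here.
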(event Custom|DelayLoop
  ;[0.15 0.15 0.15 0.5] Delay
  (Development|PrintString (Utilities|String|Append "Iteration " (Utilities|String|ToString(Integer) (stale _counter))) true true "(R=1.000000,G=0.511530,B=0.000000,A=1.000000)" 0.1)
  (Utilities|FlowControl|Delay 1.0)
  (bind _counter (Utilities|FlowControl|DoN 20)
    (:Exit
      (CallFunction|StartforLoop)
      (CallFunction|DelayLoop))))

(event Custom|StartForLoop
  (bind _array (Utilities|Array|MakeArray "(R=0.158998,G=1.000000,B=0.000000,A=1.000000)" "(R=0.072561,G=0.823958,B=0.000000,A=1.000000)" "(R=0.044497,G=0.486458,B=0.002260,A=1.000000)" "(R=0.024390,G=0.319792,B=0.000000,A=1.000000)" "(R=0.005798,G=0.115625,B=0.000000,A=1.000000)"))
  ;[0.15 0.15 0.15 0.5] For
  (for _index (range 0 (- (Utilities|Array|Length _array) 1) 2)
    (Development|PrintText (Utilities|Text|FormatText "Color index #{index}" _index) true true (Utilities|Array|Get(acopy) _array _index))))

(event Custom|StartWhileLoop
  ;[0.15 0.15 0.15 0.5] While
  (while (> (Variables|Default|GetwhileLoopCounter) 0)
    (bind _result (Math|Integer|DecrementInt (Variables|Default|GetwhileLoopCounter))
      (:%20%20
        (Development|PrintText (Utilities|Text|FormatText "There are {number} more loops left." _result) true true "(R=0.018427,G=0.000000,B=1.000000,A=1.000000)" 1.0))))
  (Development|PrintString "While loop completed." true true "(R=0.000000,G=0.660000,B=1.000000,A=1.000000)" 1.0)
  (Variables|Default|SetwhileLoopCounter 10))

(event Custom|StartForEachLoop
  ;[0.15 0.15 0.15 0.5] For Each
  (for (_array_element _array_index) (Utilities|Array|MakeArray "(R=0.158998,G=1.000000,B=0.000000,A=1.000000)" "(R=0.072561,G=0.823958,B=0.000000,A=1.000000)" "(R=0.044497,G=0.486458,B=0.002260,A=1.000000)" "(R=0.024390,G=0.319792,B=0.000000,A=1.000000)" "(R=0.005798,G=0.115625,B=0.000000,A=1.000000)")
    (Development|PrintText (Utilities|Text|FormatText "Color index #{index}" _array_index) true true _array_element)))

(event EventBeginPlay
  (Development|PrintString "LoopsAndLists BP exists.")
  (CallFunction|DelayLoop))

(fn ConstructionScript)