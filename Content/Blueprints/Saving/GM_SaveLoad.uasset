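; GM_SaveLoad is a game mode that saves and loads player stats and per-level state, loading both on BeginPlay.
; Player stats use a fixed "PlayerSave" slot, restoring stamina, health, mana and a held item found by class on the third-person character.
; Level state uses a slot named after the level, sending LoadStateMessage to each altered actor.
; Missing saves get fresh save objects; separate events write each one to disk.
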(event Custom|Load%20Player%20Stats
  (bind _returnvalue (SaveGame|DoesSaveGameExist "PlayerSave"))
  (if _returnvalue
    (bind _returnvalue_2 (SaveGame|LoadGamefromSlot "PlayerSave"))
    (bind _assg_player_stats (Utilities|Casting|CastToSG_PlayerStats _returnvalue_2))
    (Variables|Default|SetSG_PlayerStats _assg_player_stats)
    (bind _asbp_third_person_character (Utilities|Casting|CastToBP_ThirdPersonCharacter (Game|GetPlayerCharacter 0)))
    (Variables|/Game/ThirdPerson/Blueprints/BP_ThirdPersonCharacter.BP_ThirdPersonCharacter_C|SetStamina _asbp_third_person_character (Variables|/Game/Blueprints/Saving/SG_PlayerStats.SG_PlayerStats_C|GetStamina (Variables|Default|GetSG_PlayerStats)))
    (Variables|/Game/ThirdPerson/Blueprints/BP_ThirdPersonCharacter.BP_ThirdPersonCharacter_C|SetHealth _asbp_third_person_character (Variables|/Game/Blueprints/Saving/SG_PlayerStats.SG_PlayerStats_C|GetHealth (Variables|Default|GetSG_PlayerStats)))
    (Variables|/Game/ThirdPerson/Blueprints/BP_ThirdPersonCharacter.BP_ThirdPersonCharacter_C|SetMana _asbp_third_person_character (Variables|/Game/Blueprints/Saving/SG_PlayerStats.SG_PlayerStats_C|GetMana (Variables|Default|GetSG_PlayerStats)))
    (bind _returnvalue_3 (Actor|GetActorOfClass (Utilities|GetClass (Variables|/Game/Blueprints/Saving/SG_PlayerStats.SG_PlayerStats_C|GetHeldItem (Variables|Default|GetSG_PlayerStats)))))
    (Default|LoadHeldItem _asbp_third_person_character _returnvalue_3)
    (Development|PrintString "Player stats loaded." true true "(R=0.184475,G=0.000000,B=0.445201,A=1.000000)")
    (else
      (bind _returnvalue_4 (SaveGame|CreateSaveGameObject "/Game/Blueprints/Saving/SG_PlayerStats.SG_PlayerStats_C"))
      (Variables|Default|SetSG_PlayerStats _returnvalue_4))))

(event Custom|Save%20Player%20Stats
  (bind _returnvalue (SaveGame|SaveGametoSlot (Variables|Default|GetSG_PlayerStats) "PlayerSave"))
  (if _returnvalue
    (Development|PrintString "Player stats saved," true true "(R=0.184475,G=0.000000,B=0.445201,A=1.000000)")
    (else
      (Development|PrintString "Player stats could not be saved." true true "(R=0.512153,G=0.000000,B=0.022821,A=1.000000)"))))

(event Custom|Save%20Level%20State
  (bind _returnvalue (Game|GetCurrentLevelName true))
  (bind _returnvalue_2 (SaveGame|SaveGametoSlot (Variables|Default|GetSG_LevelState) _returnvalue))
  (if _returnvalue_2
    (Development|PrintString "Level state saved." true true "(R=0.184475,G=0.000000,B=0.445201,A=1.000000)")
    (else
      (Development|PrintString "Level state could not be saved." true true "(R=1.000000,G=0.002949,B=0.000000,A=1.000000)"))))

(event Custom|Load%20Level%20State
  (bind _returnvalue (Game|GetCurrentLevelName true))
  (bind _returnvalue_2 (SaveGame|DoesSaveGameExist _returnvalue))
  (if _returnvalue_2
    (bind _returnvalue_3 (SaveGame|LoadGamefromSlot _returnvalue))
    (bind _assg_level_state (Utilities|Casting|CastToSG_LevelState _returnvalue_3))
    (Variables|Default|SetSG_LevelState _assg_level_state)
    (for _array_element (Variables|/Game/Blueprints/Saving/SG_LevelState.SG_LevelState_C|GetAlteredActors (Variables|Default|GetSG_LevelState))
      (Class|BPILevelActorSaveable|LoadState(Message) (Utilities|ToObject(Interface) _array_element)))
    (else
      (bind _returnvalue_4 (SaveGame|CreateSaveGameObject "/Game/Blueprints/Saving/SG_LevelState.SG_LevelState_C"))
      (Variables|Default|SetSG_LevelState _returnvalue_4))))

(event EventBeginPlay
  (Development|PrintString "Loading Save GM" true true "(R=1.000000,G=0.615549,B=0.075234,A=1.000000)")
  (CallFunction|LoadPlayerStats)
  (CallFunction|LoadLevelState))

(fn ConstructionScript)