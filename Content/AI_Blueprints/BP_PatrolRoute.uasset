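; BP_PatrolRoute is a patrol route actor that serves world-space waypoints from a Spline component.
; GetPatrolPointLocation steps PatrolIndex by Direction and returns that spline point's location, flipping Direction at either end for back-and-forth movement.
; The upper reversal triggers only once the index reaches the point count, one past the last valid index.
; An alternative multiply-by-minus-one reversal is left unconnected, and the event graph is empty.
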(event EventBeginPlay)

(event Collision|EventActorBeginOverlap
  (params (OtherActor :type Actor%20Object%20Reference)))

(event EventTick
  (params (DeltaSeconds :type Float%20%28single-precision%29)))

(fn ConstructionScript)

(fn GetPatrolPointLocation
  (Variables|Default|SetPatrol%20Index (+ (Variables|Default|GetPatrol%20Index) (Variables|Default|GetDirection)))
  (if (>= (Variables|Default|GetPatrol%20Index) (Spline|GetNumberOfSplinePoints (Variables|Default|GetSpline))) ; At end?
    (Variables|Default|SetDirection -1) ; Reverse
    (elif (<= (Variables|Default|GetPatrol%20Index) 0) ; At beginning?
      (Variables|Default|SetDirection 1) ; Reverse
    ))
  (return (Spline|GetLocationatSplinePoint (Variables|Default|GetSpline) (Variables|Default|GetPatrol%20Index) "World")))