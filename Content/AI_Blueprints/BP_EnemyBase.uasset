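; Base enemy character with health, a melee attack, spline patrolling and hooks for aggro, investigation, walk speed and combat ranges.
; AI state drives an emissive material and colored debug text above a health readout.
; Attack sphere-traces on a montage notify, damages the player, reports it to AI perception, then signals AttackFinished.
; Patrol points ping-pong along a route spline; lethal point damage triggers an impulse ragdoll and a random Arcane Shard drop.
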(event Custom|Attack
  (bind _returnvalue (Transformation|GetActorLocation))
  ;[0.15 0.15 0.15 0.5] Attack Player
  (Animation|Montage|PlayMontage (Variables|Character|GetMesh) "/Game/CloseCombatAnimSet/Animations/InPlace/Attacks/NinjaLeftHook_Montage.NinjaLeftHook_Montage"
    (:OnNotifyBegin
      (bind (_outhit _returnvalue_2) (Collision|SphereTraceByChannel _returnvalue (+ _returnvalue (* (Transformation|GetActorForwardVector) 1.5e+02)) 5e+01 "TraceTypeQuery2" false 0 "ForDuration" true "(R=1.000000,G=0.000000,B=0.000000,A=1.000000)" "(R=0.000000,G=1.000000,B=0.000000,A=1.000000)" 1.0))
      (if _returnvalue_2
        (bind _asbp_third_person_character (Utilities|Casting|CastToBP_ThirdPersonCharacter (.HitActor (Collision|BreakHitResult _outhit)))
          (:then
            (Game|Damage|ApplyPointDamage _asbp_third_person_character (Variables|Stats|GetLightAttackDmg) (.TraceStart (Collision|BreakHitResult _outhit)) _outhit (Pawn|GetController))
            (Class|AISenseDamage|ReportDamageEvent _asbp_third_person_character self (Variables|Stats|GetLightAttackDmg) (.TraceStart (Collision|BreakHitResult _outhit)) "0, 0, 0" "None")
            (Audio|PlaySoundatLocation "/Game/Audio/Attack/punch_Cue.punch_Cue" (.TraceStart (Collision|BreakHitResult _outhit)) "0, 0, 0" 1.0 1.0 0.0 0 0 0 0))
          (:CastFailed
            (Development|PrintString "Hit something other than player." true true "(R=0.520996,G=0.000000,B=1.000000,A=1.000000)" 4.0)))
        (else
          (Development|PrintString "Missed hit." true true "(R=0.520996,G=0.000000,B=1.000000,A=1.000000)" 4.0)))
      (Default|CallAttackFinished))))

(event Custom|Get%20Aggro
  (Variables|State|SetAggro? true))

(event Custom|Lose%20Aggro
  (Variables|State|SetAggro? false))

(event Custom|Set%20Walk%20Speed
  (params (Speed :type Float%20%28double-precision%29))
  (Variables|/Script/Engine.CharacterMovementComponent|SetMaxWalkSpeed (Variables|Character|GetCharacterMovement) Speed))

(event Custom|Investigate
  (Variables|State|SetInvestigating? true))

(event Custom|Stop%20Investigation
  (Variables|State|SetInvestigating? false))

(event Custom|Set%20Material
  (params (State :type E_AIState%20Enum :default "NewEnumerator0") (Strafing? :type Boolean))
  (bind _ai_state_text (Variables|Default|GetAI%20State%20Text))
  (bind _ai_state_text_2 (Variables|Default|GetAI%20State%20Text))
  (bind _ai_state_text_3 (Variables|Default|GetAI%20State%20Text))
  (bind _ai_state_text_4 (Variables|Default|GetAI%20State%20Text))
  (bind _mesh (Variables|Character|GetMesh))
  (bind _ai_state_text_5 (Variables|Default|GetAI%20State%20Text))
  (bind _mesh_2 (Variables|Character|GetMesh))
  (switch Utilities|FlowControl|Switch|SwitchonE_AIState State
    (:NewEnumerator0
      (if (not (Variables|State|GetDead?))
        (Rendering|Material|SetMaterial _mesh_2 0 "/Game/Materials/MI_BlueEmissive.MI_BlueEmissive")
        (Rendering|Components|TextRender|SetText _ai_state_text_5 (Utilities|Text|FormatText "Waiting"))
        (Rendering|Components|TextRender|SetTextRenderColor _ai_state_text_5 (Math|Color|MakeColor 255 0 0))))
    (:NewEnumerator1
      (if (not (Variables|State|GetDead?))
        (Rendering|Material|SetMaterial _mesh_2 0 "/Game/Materials/MI_GreenEmissive.MI_GreenEmissive")
        (Rendering|Components|TextRender|SetText _ai_state_text (Utilities|Text|FormatText "Patrolling"))
        (Rendering|Components|TextRender|SetTextRenderColor _ai_state_text (Math|Color|MakeColor 0 255 0))))
    (:NewEnumerator2
      (if (not (Variables|State|GetDead?))
        (if Strafing?
          (Rendering|Material|SetMaterial _mesh 0 "/Game/Materials/MI_WhiteEmissive.MI_WhiteEmissive")
          (Rendering|Components|TextRender|SetText _ai_state_text_4 (Utilities|Text|FormatText "Strafing"))
          (Rendering|Components|TextRender|SetTextRenderColor _ai_state_text_4 (Math|Color|MakeColor 255 255 255))
          (else
            (Rendering|Material|SetMaterial _mesh 0 "/Game/Materials/MI_RedEmissive.MI_RedEmissive")
            (Rendering|Components|TextRender|SetText _ai_state_text_3 (Utilities|Text|FormatText "Attacking"))
            (Rendering|Components|TextRender|SetTextRenderColor _ai_state_text_3 (Math|Color|MakeColor 0 0 255))))))
    (:NewEnumerator3
      (if (not (Variables|State|GetDead?))
        (Rendering|Material|SetMaterial (Variables|Character|GetMesh) 0 "/Game/Materials/MI_YellowEmissive.MI_YellowEmissive")
        (Rendering|Components|TextRender|SetText _ai_state_text_2 (Utilities|Text|FormatText "Investigating"))
        (Rendering|Components|TextRender|SetTextRenderColor _ai_state_text_2 (Math|Color|MakeColor 0 180 255))))))

(event Custom|Ragdoll
  (params (Origin :type Vector))
  ;[0.15 0.15 0.15 0.5] Ragdoll on Death
  (Physics|SetSimulatePhysics (Variables|Character|GetMesh) true)
  (Physics|AddRadialImpulse (Variables|Character|GetMesh) (+ Origin "0.000000,0.000000,-50.000000") 3e+02 5e+04 "RIF_Constant" false)
  (Pawn|Components|CharacterMovement|DisableMovement (Variables|Character|GetCharacterMovement)))

(event EventBeginPlay
  (Variables|Default|SetOriginalMaterial (Rendering|Material|GetMaterial (Variables|Character|GetMesh) 0))
  (Rendering|Components|TextRender|SetText (Variables|Default|GetAI%20Health%20Text) (Utilities|Text|ToText(Float) (Variables|Stats|GetHealth) "HalfToEven")))

(event Game|Damage|EventPointDamage
  (params (Damage :type Float%20%28single-precision%29) (DamageType :type Damage%20Type%20Object%20Reference) (HitLocation :type Vector :default "0, 0, 0") (HitNormal :type Vector :default "0, 0, 0") (HitComponent :type Primitive%20Component%20Object%20Reference) (BoneName :type Name :default "None") (ShotFromDirection :type Vector :default "0, 0, 0") (InstigatedBy :type Controller%20Object%20Reference) (DamageCauser :type Actor%20Object%20Reference) (HitInfo :type Hit%20Result%20Structure%20%28by%20ref%29))
  (Development|PrintText (Utilities|Text|FormatText "{instigator} hit {damaged enemy} for {damage}." InstigatedBy HitComponent Damage) true true "(R=1.000000,G=0.447496,B=0.000000,A=1.000000)" 1e+01)
  (bind _output_get (Variables|Stats|SetHealth (- (Variables|Stats|GetHealth) Damage)))
  (Rendering|Components|TextRender|SetText (Variables|Default|GetAI%20Health%20Text) (Utilities|Text|ToText(Float) _output_get "HalfToEven"))
  (if (<= _output_get 0.0)
    (CallFunction|Ragdoll ShotFromDirection)
    (Rendering|Material|SetMaterial (Variables|Character|GetMesh) 0 "/Game/Materials/MI_FlatBlack.MI_FlatBlack")
    (Variables|State|SetDead? true)
    (if (Math|Random|RandomBool)
      (Game|SpawnActorfromClass "/Game/Blueprints/Pickups/BP_ArcaneShard.BP_ArcaneShard_C" (Math|Transform|MakeTransform (Transformation|GetActorLocation) "0, 0, 0" "1.000000,1.000000,1.000000") "Undefined" "MultiplyWithRoot" 0 0))
    (Components|DestroyComponent (Variables|Collision|GetCapsuleComponent))
    (Components|DestroyComponent (Variables|Default|GetAI%20State%20Text))
    (Components|DestroyComponent (Variables|Default|GetAI%20Health%20Text))))

(fn ConstructionScript)

(fn GetPatrolPointLocation
  (Variables|Patrol|SetPatrol%20Index (+ (Variables|Patrol|GetPatrol%20Index) (Variables|Patrol|GetDirection)))
  (if (>= (Variables|Patrol|GetPatrol%20Index) (- (Spline|GetNumberOfSplinePoints (Variables|/Game/AI_Blueprints/BP_PatrolRoute.BP_PatrolRoute_C|GetSpline (Variables|Patrol|GetPatrolRoute))) 1)) ; At end?
    (Variables|Patrol|SetDirection -1) ; Reverse
    (elif (<= (Variables|Patrol|GetPatrol%20Index) 0) ; At beginning?
      (Variables|Patrol|SetDirection 1) ; Reverse
    ))
  (return (Spline|GetLocationatSplinePoint (Variables|/Game/AI_Blueprints/BP_PatrolRoute.BP_PatrolRoute_C|GetSpline (Variables|Patrol|GetPatrolRoute)) (Variables|Patrol|GetPatrol%20Index) "World")))

(fn GetIdealRange
  (return (Variables|Stats|GetAttack%20Range) (Variables|Stats|GetStrafe%20Range)))