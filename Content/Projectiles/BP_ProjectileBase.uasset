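; Base projectile Blueprint that flies toward a target location and destroys itself on contact.
; On BeginPlay it sets the ProjectileMovement velocity from the direction to TargetLocation scaled by Speed, then activates the component.
; Its collision sphere destroys the actor on any blocking hit, or on overlap with any actor other than its Instigator.
; It applies no damage itself.
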(event OnComponentBeginOverlap(SphereCollision)
  (params (OverlappedComponent :type Primitive%20Component%20Object%20Reference) (OtherActor :type Actor%20Object%20Reference) (OtherComp :type Primitive%20Component%20Object%20Reference) (OtherBodyIndex :type Integer) (bFromSweep :type Boolean) (SweepResult :type Hit%20Result%20Structure%20%28by%20ref%29))
  (if (!= OtherActor (Variables|Actor|GetInstigator)) ; Is the actor NOT myself?
    (Actor|DestroyActor)))

(event OnComponentHit(SphereCollision)
  (params (HitComponent :type Primitive%20Component%20Object%20Reference) (OtherActor :type Actor%20Object%20Reference) (OtherComp :type Primitive%20Component%20Object%20Reference) (NormalImpulse :type Vector :default "0, 0, 0") (Hit :type Hit%20Result%20Structure%20%28by%20ref%29))
  (Actor|DestroyActor) ; Overlapping Block; destroy
)

(event EventBeginPlay
  (bind _projectilemovement (Variables|Default|GetProjectileMovement))
  (Variables|/Script/Engine.MovementComponent|SetVelocity _projectilemovement (* (Math|Vector|GetUnitDirection(Vector) (Transformation|GetActorLocation) (Variables|ProjectileSettings|GetTargetLocation)) (Variables|ProjectileSettings|GetSpeed)))
  (Components|Activation|Activate _projectilemovement false))

(fn ConstructionScript)